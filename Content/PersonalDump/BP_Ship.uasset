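; BP_Ship is a pilotable physics ship that a player can enter and exit, passing possession and toggling gravity.
; BeginPlay shifts the center of mass toward the PhysicsThruster in X/Y, and axis inputs apply pitch and roll torque.
; The TakeOff axis drives mass- and tilt-compensated lift until interpolated Thrust reaches a threshold, then sets forward velocity directly.
; Holding Boost raises MaxThrust; its instant-kick branch never runs because it compares constant zeros.
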(event `InputAction|EnterExitShip`
  (params (Key :type "Key Structure"))
  (:`Pressed`
    (`self.Exit`)))

(event `InputAxis|TakeOff`
  (params (AxisValue :type "Float (single-precision)"))
  (bind (_returnvalue_x _returnvalue_y _returnvalue_z) (`KismetMathLibrary.BreakVector` (`self.GetActorUpVector`)))
  (if (>= (`self.Thrust`) 100.0)
    (`PrimitiveComponent.SetPhysicsLinearVelocity` (`self.Ship`) (`self.ForwardVelocity`) false "None")
    (else
      (set `PhysicsThrusterComponent.ThrustStrength` (* (/ (* AxisValue 500.0) _returnvalue_z) (`PrimitiveComponent.GetMass` (`self.Ship`))) (`self.PhysicsThruster`)))))

(event `self.ReceiveBeginPlay`
  (bind _ship (`self.Ship`))
  (bind (_returnvalue_x _returnvalue_y) (`KismetMathLibrary.BreakVector` (`KismetMathLibrary.GreaterGreater_VectorRotator` (- (`SceneComponent.K2_GetComponentLocation` (`self.PhysicsThruster`)) (`PrimitiveComponent.GetCenterOfMass` _ship "None")) (`KismetMathLibrary.NegateRotator` (`SceneComponent.K2_GetComponentRotation` _ship)))))
  (`PrimitiveComponent.SetCenterOfMass` (`self.Ship`) (`KismetMathLibrary.MakeVector` _returnvalue_x _returnvalue_y) "None"))

(event `InputAxis|MoveUp`
  (params (AxisValue :type "Float (single-precision)"))
  (`PrimitiveComponent.AddTorqueInDegrees` (`self.Ship`) (* (`SceneComponent.GetRightVector` (`self.Ship`)) (* AxisValue (`self.ForwardTorquePower`))) "None" true))

(event `InputAxis|MoveRight`
  (params (AxisValue :type "Float (single-precision)"))
  (`PrimitiveComponent.AddTorqueInDegrees` (`self.Ship`) (* (`SceneComponent.GetForwardVector` (`self.Ship`)) (* AxisValue (`self.RotateTorque`))) "None" true))

(event `InputAxis|Thrust`
  (params (AxisValue :type "Float (single-precision)"))
  (`|ExecutionSequence`
    (:`then_0`
      (if (not (`KismetMathLibrary.NearlyEqual_FloatFloat` AxisValue 0.0 0.1))
        (set `self.Thrust` (`KismetMathLibrary.FInterpTo` (`self.Thrust`) (`KismetMathLibrary.Lerp` 0.0 (`self.MaxThrust`) (/ (+ AxisValue 1.0) 2.0)) (`GameplayStatics.GetWorldDeltaSeconds`) 1.0))))
    (:`then_1`
      (set `self.ForwardVelocity` (* (`SceneComponent.GetForwardVector` (`self.Ship`)) (`self.Thrust`))))))

(event `InputAction|Boost`
  (params (Key :type "Key Structure"))
  (:`Pressed`
    (set `self.MaxThrust` 10000.0)
    (`|ExecutionSequence`
      (:`then_0`
        (if (not (`KismetMathLibrary.NearlyEqual_FloatFloat` 0.0 0.0 0.1))
          (bind _output_get (set `self.Thrust` (* (`KismetMathLibrary.FInterpTo` (`self.Thrust`) (`KismetMathLibrary.Lerp` 0.0 (`self.MaxThrust`) (/ (+ 0.0 1.0) 2.0)) (`GameplayStatics.GetWorldDeltaSeconds`) 1.0) 5.0)))
          (`KismetSystemLibrary.PrintString` (`KismetStringLibrary.Conv_DoubleToString` _output_get))))
      (:`then_1`
        (set `self.ForwardVelocity` (* (`SceneComponent.GetForwardVector` (`self.Ship`)) (`self.Thrust`))))))
  (:`Released`
    (set `self.MaxThrust` 1000.0)))

(fn `Enter`
  (params (Player :type "/Game/TopDown/Blueprints/BP_TopDownCharacter Object Reference") (`Exit Delegate` :type "Delegate (by ref)"))
  (add `self.OnExited` `Exit Delegate`)
  (bind _output_get (set `self.Occupant` Player))
  (`Controller.Possess` (`self.GetController` _output_get) self)
  (`self.K2_AttachToActor` (`self.Occupant`) self "Pilot" "SnapToTarget" "SnapToTarget" "SnapToTarget" true)
  (`PrimitiveComponent.SetEnableGravity` (`self.Ship`) false))

(fn `Exit`
  (bind _occupant (`self.Occupant`))
  (`self.K2_DetachFromActor` _occupant "KeepWorld" "KeepWorld" "KeepWorld")
  (`self.K2_SetActorLocation` _occupant (`SceneComponent.K2_GetComponentLocation` (`self.Box`)) false false)
  (`Controller.Possess` (`self.GetController`) _occupant)
  (`PrimitiveComponent.SetEnableGravity` (`self.Ship`) true)
  (`self.OnExited`))

(fn `UserConstructionScript`)